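; Sample base player character Blueprint that assembles a modular body from separate Head, UpperBody, LowerBody and Shoes components.
; The construction script sets the main Mesh as leader pose component for each part, so all four follow its animated pose.
; The event graph holds only disabled placeholder events and adds no gameplay logic.
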(fn `UserConstructionScript`
  (`SkinnedMeshComponent.SetLeaderPoseComponent` (`self.Head`) (`self.Mesh`) false false)
  (`SkinnedMeshComponent.SetLeaderPoseComponent` (`self.UpperBody`) (`self.Mesh`) false false)
  (`SkinnedMeshComponent.SetLeaderPoseComponent` (`self.LowerBody`) (`self.Mesh`) false false)
  (`SkinnedMeshComponent.SetLeaderPoseComponent` (`self.Shoes`) (`self.Mesh`) false false))