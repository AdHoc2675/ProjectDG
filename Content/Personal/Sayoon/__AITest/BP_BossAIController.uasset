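; Test AI controller for the Kashapa boss that starts its behavior tree, BT_Kashapa, on BeginPlay with network authority.
; The Possess and perception update events are empty.
; Disconnected logic holds a State Tree alternative (ST_Kashapa) and a perception handler that would write sensed Team.Player actors, identified by gameplay tag, to the blackboard as target actor and location.
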(event `self.ReceiveBeginPlay`
  (`/Engine/EditorBlueprintResources/ActorMacros.Switch Has Authority`
    (:`Authority`
      (`self.RunBehaviorTree` "/Game/Personal/Sayoon/__AITest/Kashapa/Kashapa_V1/BT_Kashapa.BT_Kashapa"))))

(event `self.ReceivePossess`
  (params (PossessedPawn :type "Pawn Object Reference")))

(event `self.EnemyPerceptionComponent.OnTargetPerceptionUpdated`
  (params (Actor :type "Actor Object Reference") (Stimulus :type "AIStimulus Structure")))

(fn `UserConstructionScript`)