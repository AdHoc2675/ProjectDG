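; Test Blueprint for the Kashapa V2 boss character, holding a basic attack and an unfinished combo system.
; Attack sets ComboDecide on the authority and plays the Skill03 montage, which reuses a V1 animation asset.
; ComboAttack, BeginPlay and Tick are empty.
; A looping server-side attack timer and a montage jump between two skill sections are present but disconnected, so nothing in this graph triggers Attack.
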(event `self.ReceiveBeginPlay`)

(event `Attack`
  (`/Engine/EditorBlueprintResources/ActorMacros.Switch Has Authority`
    (:`Authority`
      (set `self.ComboDecide` true))
    (:`Remote`
      _))
  (`self.PlayAnimMontage` "/Game/Personal/Sayoon/__AITest/Kashapa/Kashapa_V1/Ani/AM_Kashapa_V1_Skill03.AM_Kashapa_V1_Skill03"))

(event `ComboAttack`
  (params (bPickA :type Boolean)))

(event `self.ReceiveTick`
  (params (DeltaSeconds :type "Float (single-precision)")))

(fn `UserConstructionScript`)