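; Static mesh actor that dissolves with a matching Niagara effect, driven by overlaps on its box component.
; The construction script creates a dynamic material instance, assigns the Niagara asset, and feeds both the same dissolve amount, world position, texture and UV values.
; Box overlap plays a timeline and end overlap reverses it, remapping its value between the start and end amounts to update material and particles in sync.
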(event `self.ReceiveBeginPlay`
  (bind _dissolvestart (`self.DissolveStart`))
  (`NiagaraComponent.SetVariableFloat` (`self.Niagara`) "DissolveAmount" _dissolvestart)
  (`MaterialInstanceDynamic.SetScalarParameterValue` (`self.DynamicDissolveMaterial`) "DissolveAmount" _dissolvestart))

(event `self.Box.OnComponentBeginOverlap`
  (params (OverlappedComponent :type "PrimitiveComponent Object Reference") (OtherActor :type "Actor Object Reference") (OtherComp :type "PrimitiveComponent Object Reference") (OtherBodyIndex :type Integer) (bFromSweep :type Boolean) (SweepResult :type "HitResult Structure (by ref)"))
  (bind (_direction _dissolveamount) (`Timeline|DissolveTimeline` :!label _label)
    (:`Update`
      (bind _returnvalue (`KismetMathLibrary.MapRangeClamped` _dissolveamount 0.0 1.0 (`self.DissolveEnd`) (`self.DissolveStart`)))
      (`NiagaraComponent.SetVariableFloat` (`self.Niagara`) "DissolveAmount" _returnvalue)
      (`MaterialInstanceDynamic.SetScalarParameterValue` (`self.DynamicDissolveMaterial`) "DissolveAmount" _returnvalue))))

(event `self.Box.OnComponentEndOverlap`
  (params (OverlappedComponent :type "PrimitiveComponent Object Reference") (OtherActor :type "Actor Object Reference") (OtherComp :type "PrimitiveComponent Object Reference") (OtherBodyIndex :type Integer))
  (goto _label :!via `Reverse`))

(fn `UserConstructionScript`
  (bind _dissolvetexture (`self.DissolveTexture`))
  (bind _dissolveamount (`self.DissolveAmount`))
  (bind _dynamicdissolvematerial (`self.DynamicDissolveMaterial`))
  (bind _dissolvetextureuv (`self.DissolveTextureUV`))
  (bind _niagara (`self.Niagara`))
  (bind (_x _y) (`KismetMathLibrary.BreakVector2D` _dissolvetextureuv))
  (bind _returnvalue (`SceneComponent.K2_GetComponentLocation` (`self.DissolvePosition`)))
  (bind _returnvalue_2 (`PrimitiveComponent.CreateDynamicMaterialInstance` (`self.StaticMesh`) 0 (`self.DissolveMaterial`) "None"))
  (set `self.DynamicDissolveMaterial` _returnvalue_2)
  (`NiagaraComponent.SetAsset` (`self.Niagara`) (`self.SetDissolveNiagara`) true)
  (`NiagaraComponent.SetVariableFloat` _niagara "DissolveAmount" _dissolveamount)
  (`MaterialInstanceDynamic.SetScalarParameterValue` _dynamicdissolvematerial "DissolveAmount" _dissolveamount)
  (`MaterialInstanceDynamic.SetVectorParameterValue` _dynamicdissolvematerial "Position" (`KismetMathLibrary.Conv_VectorToLinearColor` _returnvalue))
  (`NiagaraComponent.SetVariableVec3` (`self.Niagara`) "Position" _returnvalue)
  (`NiagaraComponent.SetVariableTexture` _niagara "DissolveTexture" _dissolvetexture)
  (`MaterialInstanceDynamic.SetTextureParameterValue` _dynamicdissolvematerial "DissolveTexture" _dissolvetexture)
  (`MaterialInstanceDynamic.SetVectorParameterValue` _dynamicdissolvematerial "DissolveTextureUV" (`KismetMathLibrary.Conv_VectorToLinearColor` (`KismetMathLibrary.MakeVector` _x _y)))
  (`NiagaraComponent.SetVariableVec2` _niagara "DissolveTextureUV" _dissolvetextureuv))