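; Sword actor Blueprint that attaches Niagara effects to its SMSword mesh on BeginPlay.
; It spawns NS_SwordEffect2 at an offset snapped to the mesh, plus NS_SwordEffect2_Trails centered between the trail-bottom and trail-top sockets.
; The trail's Z axis follows the line between those sockets, and their distance sets its TrailSize parameter, fitting the trail to the socket span.
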(event `self.ReceiveBeginPlay`
  (bind _sm_sword (`self.SM_sword`))
  (bind _returnvalue (`SceneComponent.GetSocketLocation` _sm_sword "trail-top"))
  (bind _returnvalue_2 (`SceneComponent.GetSocketLocation` _sm_sword "trail-bottom"))
  (bind _returnvalue_3 (- _returnvalue _returnvalue_2))
  (`NiagaraFunctionLibrary.SpawnSystemAttached` "/Game/Assets/SwordEffects/Particles/NS_SwordEffect2.NS_SwordEffect2" _sm_sword "None" (0.0 0.0 20.398507) (struct) "SnapToTarget")
  (bind _returnvalue_4 (`NiagaraFunctionLibrary.SpawnSystemAttached` "/Game/Assets/SwordEffects/Particles/NS_SwordEffect2_Trails.NS_SwordEffect2_Trails" _sm_sword "None" (/ (+ _returnvalue_2 _returnvalue) 2.0) (`KismetMathLibrary.MakeRotFromZ` _returnvalue_3) "KeepWorldPosition"))
  (`FXSystemComponent.SetFloatParameter` _returnvalue_4 "TrailSize" (`KismetMathLibrary.VSize` _returnvalue_3)))

(fn `UserConstructionScript`)