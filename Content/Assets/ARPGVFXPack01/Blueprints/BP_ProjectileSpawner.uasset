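; BP_ProjectileSpawner is a looping spawner that repeatedly fires configurable VFX projectiles from its location, apparently for showcasing the effects pack.
; On BeginPlay it fires once, then a looping timer re-runs the spawn event every LoopTime.
; Each spawned BP_ProjectileMaster receives the spawner's muzzle, projectile and impact effects, offsets and destroy delay, plus a velocity along world +X scaled by ProjectileSpeed.
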(event `self.ReceiveBeginPlay`
  (`self.SpawnProjectileVFX`)
  (`KismetSystemLibrary.K2_SetTimerDelegate` (delegate `SpawnProjectileVFX`) (`self.LoopTime`) true))

(event `SpawnProjectileVFX`
  (bind _returnvalue (`|SpawnActorFromClass` "/Game/Assets/ARPGVFXPack01/Blueprints/BP_ProjectileMaster.BP_ProjectileMaster_C" (`KismetMathLibrary.MakeTransform` (`self.K2_GetActorLocation`)) "Undefined" "OverrideRootScale" null null))
  (bind _output_get (set `self.SpawnedProjectile` _returnvalue))
  (`/Engine/EditorBlueprintResources/StandardMacros.IsValid` _output_get
    (:`Is Valid`
      (`|ExecutionSequence`
        (:`then_0`
          (set `/Game/Assets/ARPGVFXPack01/Blueprints/BP_ProjectileMaster.MuzzleFlash` (`self.Muzzle Flash`) (`self.SpawnedProjectile`))
          (`NiagaraComponent.SetAsset` (`/Game/Assets/ARPGVFXPack01/Blueprints/BP_ProjectileMaster.Projectile` (`self.SpawnedProjectile`)) (`self.MainProjectile`) true)
          (set `/Game/Assets/ARPGVFXPack01/Blueprints/BP_ProjectileMaster.Impack` (`self.Impack`) (`self.SpawnedProjectile`)))
        (:`then_1`
          ;[0 0 0] set velocity
          (set `MovementComponent.Velocity` (* (1.0 0.0 0.0) (`self.ProjectileSpeed`)) (`/Game/Assets/ARPGVFXPack01/Blueprints/BP_ProjectileMaster.ProjectileMovement` (`self.SpawnedProjectile`))))
        (:`then_2`
          (set `/Game/Assets/ARPGVFXPack01/Blueprints/BP_ProjectileMaster.Muzzle Offset` (`self.Muzzle Offset`) (`self.SpawnedProjectile`)))
        (:`then_3`
          (set `/Game/Assets/ARPGVFXPack01/Blueprints/BP_ProjectileMaster.Impack Offset` (`self.Impack Offset`) (`self.SpawnedProjectile`)))
        (:`then_4`
          (set `/Game/Assets/ARPGVFXPack01/Blueprints/BP_ProjectileMaster.ProjectileDestoryDelay` (`self.Projectile Destory Delay`) (`self.SpawnedProjectile`)))))))

(fn `UserConstructionScript`)