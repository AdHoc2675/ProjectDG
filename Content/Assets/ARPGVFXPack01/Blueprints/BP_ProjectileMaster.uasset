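; Master projectile Blueprint for the ARPG VFX pack that plays muzzle flash, projectile and impact Niagara effects.
; Shortly after BeginPlay it spawns the muzzle effect at an offset through a shared SpawnVFX helper.
; When its Box overlaps a BP_BlockBox, it stops moving and spawns the impact effect.
; It also sets Niagara variables to kill main meshes and zero the spawn rate, then destroys itself after a delay.
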(event `self.ReceiveBeginPlay`
  (`KismetSystemLibrary.Delay` 0.02)
  (`self.SpawnVFX` (`self.MuzzleFlash`) (`self.Muzzle Offset`)))

(event `self.Box.OnComponentBeginOverlap`
  (params (OverlappedComponent :type "PrimitiveComponent Object Reference") (OtherActor :type "Actor Object Reference") (OtherComp :type "PrimitiveComponent Object Reference") (OtherBodyIndex :type Integer) (bFromSweep :type Boolean) (SweepResult :type "HitResult Structure (by ref)"))
  (cast `/Game/Assets/ARPGVFXPack01/Blueprints/BP_BlockBox` OtherActor)
  (`MovementComponent.StopMovementImmediately` (`self.ProjectileMovement`))
  (`NiagaraComponent.SetVariableBool` (`self.Projectile`) "KillMainMeshs" true)
  (`NiagaraComponent.SetVariableFloat` (`self.Projectile`) "SpawnRateMul" 0.0)
  (`self.SpawnVFX` (`self.Impack`) (`self.Impack Offset`))
  (`KismetSystemLibrary.Delay` (`self.ProjectileDestoryDelay`))
  (`self.K2_DestroyActor`))

(fn `SpawnVFX`
  (params (SpawnVFX :type "NiagaraSystem Object Reference") (LocationOffset :type "Vector Structure"))
  (`/Engine/EditorBlueprintResources/StandardMacros.IsValid` SpawnVFX
    (:`Is Valid`
      (`NiagaraFunctionLibrary.SpawnSystemAtLocation` SpawnVFX (+ LocationOffset (`self.K2_GetActorLocation`))))))

(fn `UserConstructionScript`)