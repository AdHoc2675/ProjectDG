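; Actor Blueprint in the ARPG VFX pack that replays a configurable Niagara effect at a fixed interval.
; BeginPlay spawns the system once and starts a looping timer set by TimeReplay, whose Timeout event spawns it again on each tick of the timer.
; Each spawn uses the actor's location plus PositionOffset, the actor's rotation and the configured Scale.
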(event `self.ReceiveBeginPlay`
  (`KismetSystemLibrary.K2_SetTimer` null "Timeout" (`self.Time_Replay`) true)
  (`NiagaraFunctionLibrary.SpawnSystemAtLocation` (`self.NiagaraSystem`) (+ (`self.K2_GetActorLocation`) (`self.PositionOffset`)) (`self.K2_GetActorRotation`) (`self.Scale`)))

(event `Timeout`
  (`NiagaraFunctionLibrary.SpawnSystemAtLocation` (`self.NiagaraSystem`) (+ (`self.K2_GetActorLocation`) (`self.PositionOffset`)) (`self.K2_GetActorRotation`) (`self.Scale`)))

(fn `UserConstructionScript`)